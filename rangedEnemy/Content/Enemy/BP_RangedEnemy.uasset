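; BP_RangedEnemy is a bow-wielding enemy that reports equal attack and defend ranges through GetIdealRange.
; On BeginPlay it spawns a BP_Bow and attaches it to a left-hand socket on its mesh.
; Attack plays a bow-shot montage whose notify line-traces from the bow to the AI controller's target.
; An unobstructed trace only prints a damage message; montage completion or interruption signals the attack's end.
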(event `self.ReceiveBeginPlay`
  (`self.WeildWeapon`))

(event `/Game/Enemy/AI/BPI_EnemyAI.WeildWeapon`
  (bind _returnvalue (`|SpawnActorFromClass` "/Game/Enemy/Weapons/BPs/BP_Bow.BP_Bow_C" (`KismetMathLibrary.MakeTransform` (0.0 0.0 0.0)) "Undefined" "MultiplyWithRoot" null null))
  (bind _output_get (set `self.WeaponActor` _returnvalue))
  (`self.K2_AttachToComponent` _output_get (`self.Mesh`) "hand_l_BowSocket" "SnapToTarget" "SnapToTarget" "SnapToTarget" true)
  (set `self.IsWieldingWeapon` true))

(event `/Game/Enemy/AI/BPI_EnemyAI.Attack`
  (bind _notifyname (`|PlayMontage` (`self.Mesh`) "/Game/Enemy/Animation/Montage/AM_BowShot.AM_BowShot")
    (:`OnCompleted`
      (`self.OnAttackEnd` :!label _label))
    (:`OnInterrupted`
      (goto _label))
    (:`OnNotifyBegin`
      (switch `name` _notifyname
        (:`Shoot`
          (bind _asaic_enemy_base (cast `/Game/Enemy/AI/AIC_EnemyBase` (`AIBlueprintHelperLibrary.GetAIController` self)))
          (bind _attack_target (`/Game/Enemy/AI/AIC_EnemyBase.Attack Target` _asaic_enemy_base)
            (:`then`
              (bind (_outhit _returnvalue) (`KismetSystemLibrary.LineTraceSingle` :`Start` (`self.K2_GetActorLocation` (`self.WeaponActor`)) :`End` (`self.K2_GetActorLocation` _attack_target) :`TraceChannel` "TraceTypeQuery1" :`DrawDebugType` "ForDuration"))
              (if (not _returnvalue)
                (`KismetSystemLibrary.PrintString` "Damaged")))
            (:`else`
              (`KismetSystemLibrary.PrintString` "invalid"))))))))

(fn `GetIdealRange`
  (returns (AttackRadius :type "Float (double-precision)") (DefendRadius :type "Float (double-precision)"))
  (return 600.0 600.0))

(fn `UserConstructionScript`
  (`parent.UserConstructionScript`))